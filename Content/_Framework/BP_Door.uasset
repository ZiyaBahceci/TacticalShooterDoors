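; BP_Door is a breachable door that can be locked, kicked, peeked through, opened or booby-trapped.
; The server randomizes lock, kick toughness and bomb on BeginPlay, with an OnRep removing the trap component when no bomb is present.
; Kicks reduce toughness until breach, while unlocking allows peeking or opening, both animated by timelines rotating the mesh.
; Breaching detonates an undisarmed trap with sound and particles, and the finished swing increments GS_GameState's DoorsBreached.
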(event `Unlock`
  ;[1 1 1] Unlocking (runs when lock is picked)
  (set `self.bLocked` false)
  (set `self.Toughness` 0))

(event `self.ReceiveBeginPlay`
  ;[0 0.9314 1] Door Randomization
  ;;[1 1 1] Connect for randomization
  (`self.SR_Randomize`))

(event `SR_Randomize`
  ;[0 0.9314 1] Door Randomization
  (`/Engine/EditorBlueprintResources/ActorMacros.Switch Has Authority`
    (:`Authority`
      (set `self.bLocked` (`KismetMathLibrary.RandomBool`))
      (set `self.bHasBomb` (`KismetMathLibrary.RandomBool`))
      (if (`self.bLocked`)
        (set `self.Toughness` (`KismetMathLibrary.RandomIntegerInRange` 1 3))))))

(event `KickDoor`
  ;[1 1 1] Controls opening and kicking (breaching in general)
  (bind _result (`/Engine/EditorBlueprintResources/StandardMacros.DecrementInt` (`self.Toughness`))
    (:`  `
      (if (<= (`KismetMathLibrary.Clamp` _result 0 3) 0)
        (`self.Breach`)))))

(event `Breach`
  ;[1 1 1] Controls opening and kicking (breaching in general)
  (set `self.bLocked` false)
  (set `self.Toughness` 0)
  (set `self.bBreached` true :!label _label)
  (if (`self.bHasBomb`)
    (`self.ActivateTrap`))
  (if (`self.bPeeked`)
    (`|ExecutionSequence`
      (:`then_0`
        (bind (_direction _opendoorcurve) (`Timeline|DoorOpenTimeline` :`NewTime` 0.105 :!via `SetNewTime` :!label _label_2)
          (:`Update`
            (`SceneComponent.K2_SetRelativeRotation` (`self.SM_Door`) (`KismetMathLibrary.MakeRotator` 0.0 0.0 _opendoorcurve) false false))
          (:`Finished`
            (bind _asgs_game_state (cast `/Game/_Framework/GS_GameState` (`GameplayStatics.GetGameState`)))
            (`/Engine/EditorBlueprintResources/StandardMacros.IncrementInt` (`/Game/_Framework/GS_GameState.DoorsBreached` _asgs_game_state)))))
      (:`then_1`
        (goto _label_2)))
    (else
      (goto _label_2))))

(event `TryOpen`
  ;[1 1 1] Controls opening and kicking (breaching in general)
  (if (and (not (`self.bLocked`)) (<= (`self.Toughness`) 0))
    (goto _label)))

(event `Peek`
  ;[1 1 1] Controls Peeking
  (if (and (not (`self.bLocked`)) (<= (`self.Toughness`) 0) (not (`self.bBreached`)))
    (set `self.bPeeked` true)
    (bind (_direction _opendoorcurve) (`Timeline|Timeline`)
      (:`Update`
        (`SceneComponent.K2_SetRelativeRotation` (`self.SM_Door`) (`KismetMathLibrary.MakeRotator` 0.0 0.0 _opendoorcurve) false false)))))

(event `DisarmTrap`
  ;[1 1 1] Disarm Trap
  (set `self.BombDisarmed` true)
  (bind _asbp_door_trap (cast `/Game/_Framework/BP_DoorTrap` (`ChildActorComponent.ChildActor` (`self.BP_DoorTrap`))))
  (bind _sm_statue (`/Game/_Framework/BP_DoorTrap.SM_Statue` _asbp_door_trap))
  (`PrimitiveComponent.SetMaterial` _sm_statue 0 "/Engine/EngineDebugMaterials/BoneWeightMaterial.BoneWeightMaterial")
  (`PrimitiveComponent.SetMaterial` _sm_statue 1 "/Engine/EditorMaterials/GeometryCollection/SelectedGeometryMaterial.SelectedGeometryMaterial"))

(event `ActivateTrap`
  (bind _returnvalue (`self.K2_GetActorLocation`))
  (bind _bp_doortrap (`self.BP_DoorTrap`))
  ;[1 1 1] Set off trap
  (if (not (`self.BombDisarmed`))
    (`GameplayStatics.PlaySoundAtLocation` "/Game/StarterContent/Audio/Explosion01.Explosion01" _returnvalue (struct) 1.0 1.0 0.0 null null null null)
    (`GameplayStatics.SpawnEmitterAtLocation` "/Game/StarterContent/Particles/P_Explosion.P_Explosion" _returnvalue)
    (`/Engine/EditorBlueprintResources/StandardMacros.IsValid` _bp_doortrap
      (:`Is Valid`
        (`ActorComponent.K2_DestroyComponent` _bp_doortrap)))))

(fn `OnRep_bHasBomb`
  (if (not (`self.bHasBomb`))
    (`ActorComponent.K2_DestroyComponent` (`self.BP_DoorTrap`))))

(fn `OnRep_bLocked`
  (if (`self.bLocked`)
    _))

(fn `OnRep_RandomSeed`)

(fn `OnRep_Toughness`)

(fn `UserConstructionScript`)