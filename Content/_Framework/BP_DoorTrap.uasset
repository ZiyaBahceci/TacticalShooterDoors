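; BP_DoorTrap is an explosive trap actor, noted as unused because child actors cause replication issues.
; Activate plays an explosion sound and particle effect at the actor's location, then destroys the actor, unless the trap is disarmed.
; Disarm sets the IsDisarmed flag and swaps both statue material slots to other materials.
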(event `Activate`
  (bind (_returnvalue_location _returnvalue_rotation _returnvalue_scale) (`KismetMathLibrary.BreakTransform` (`self.GetTransform`)))
  ;[1 0 0] Unused because child actors cause replication issues
  (if (not (`self.IsDisarmed`))
    (`GameplayStatics.PlaySoundAtLocation` "/Game/StarterContent/Audio/Explosion01.Explosion01" (`self.K2_GetActorLocation`) (struct) 1.0 1.0 0.0 null null null null)
    (`GameplayStatics.SpawnEmitterAtLocation` "/Game/StarterContent/Particles/P_Explosion.P_Explosion" _returnvalue_location _returnvalue_rotation _returnvalue_scale)
    (`self.K2_DestroyActor`)))

(event `Disarm`
  (bind _sm_statue (`self.SM_Statue`))
  ;[1 0 0] Unused because child actors cause replication issues
  (set `self.IsDisarmed` true)
  (`PrimitiveComponent.SetMaterial` _sm_statue 0 "/Engine/EngineDebugMaterials/BoneWeightMaterial.BoneWeightMaterial")
  (`PrimitiveComponent.SetMaterial` _sm_statue 1 "/Engine/EditorMaterials/GeometryCollection/SelectedGeometryMaterial.SelectedGeometryMaterial"))

(fn `UserConstructionScript`)